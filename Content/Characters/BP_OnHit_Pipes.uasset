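; BP_OnHit_Pipes is a pipes hit trigger that destroys every BP_Explosive_Glass actor in the level and plays a grenade explosion sound at a fixed world position.
; Hits on OnHit_Trigger or Box run duplicated destroy loops that also print each actor's name.
; The damage event joins the first loop but binds itself only inside its own body.
; The CargoDestroy tag lookup result is unused.
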(event OnComponentHit(OnHit_Trigger)
  (params (HitComponent :type Primitive%20Component%20Object%20Reference) (OtherActor :type Actor%20Object%20Reference) (OtherComp :type Primitive%20Component%20Object%20Reference) (NormalImpulse :type Vector :default "0, 0, 0") (Hit :type Hit%20Result%20Structure%20%28by%20ref%29))
  (Actor|GetAllActorswithTag "CargoDestroy")
  (bind _outactors (Actor|GetAllActorsOfClass "/Game/ResearchMegaPack/ResearchUnderground/Materials/MasterMaterial/BP_Explosive_Glass.BP_Explosive_Glass_C"))
  (for _array_element _outactors
    (Development|PrintString (Utilities|GetDisplayName _array_element))
    (Actor|DestroyActor _array_element))
  (Audio|PlaySoundatLocation "/Game/MilitaryWeapDark/Sound/GrenadeLauncher/GrenadeLauncher_Explosion_Cue.GrenadeLauncher_Explosion_Cue" "-3738.000000,1237.000000,0.000000" "0, 0, 0" 1.0 1.0 0.0 0 0 0 0))

(event OnComponentHit(Box)
  (params (HitComponent :type Primitive%20Component%20Object%20Reference) (OtherActor :type Actor%20Object%20Reference) (OtherComp :type Primitive%20Component%20Object%20Reference) (NormalImpulse :type Vector :default "0, 0, 0") (Hit :type Hit%20Result%20Structure%20%28by%20ref%29))
  (bind _outactors (Actor|GetAllActorsOfClass "/Game/ResearchMegaPack/ResearchUnderground/Materials/MasterMaterial/BP_Explosive_Glass.BP_Explosive_Glass_C"))
  (for _array_element _outactors
    (Development|PrintString (Utilities|GetDisplayName _array_element))
    (Actor|DestroyActor _array_element))
  (Audio|PlaySoundatLocation "/Game/MilitaryWeapDark/Sound/GrenadeLauncher/GrenadeLauncher_Explosion_Cue.GrenadeLauncher_Explosion_Cue" "-3738.000000,1237.000000,0.000000" "0, 0, 0" 1.0 1.0 0.0 0 0 0 0))

(event Custom|OnTakeAnyDamage_Event
  (params (DamagedActor :type Actor%20Object%20Reference) (Damage :type Float%20%28single-precision%29) (DamageType :type Damage%20Type%20Object%20Reference) (InstigatedBy :type Controller%20Object%20Reference) (DamageCauser :type Actor%20Object%20Reference))
  (EventDispatchers|AssignOnTakeAnyDamage (delegate Custom|OnTakeAnyDamage_Event))
  (bind _outactors (Actor|GetAllActorsOfClass "/Game/ResearchMegaPack/ResearchUnderground/Materials/MasterMaterial/BP_Explosive_Glass.BP_Explosive_Glass_C"))
  (for _array_element _outactors
    (Development|PrintString (Utilities|GetDisplayName _array_element))
    (Actor|DestroyActor _array_element))
  (Audio|PlaySoundatLocation "/Game/MilitaryWeapDark/Sound/GrenadeLauncher/GrenadeLauncher_Explosion_Cue.GrenadeLauncher_Explosion_Cue" "-3738.000000,1237.000000,0.000000" "0, 0, 0" 1.0 1.0 0.0 0 0 0 0))

(event EventBeginPlay)

(event Collision|EventActorBeginOverlap
  (params (OtherActor :type Actor%20Object%20Reference)))

(event EventTick
  (params (DeltaSeconds :type Float%20%28single-precision%29)))

(fn ConstructionScript)