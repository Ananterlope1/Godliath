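; BP_PlayerCharacter is the player character Blueprint, handling input mode setup and opening the pause menu.
; BeginPlay switches the player controller to game-only input.
; Pressing P creates WBP_PauseMenu once and caches it, then shows the cursor, switches to UI-only input focused on the menu, adds it to the viewport and pauses the game.
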(event EventBeginPlay
  (Input|SetInputModeGameOnly (Game|GetPlayerController 0) false))

(event Collision|EventActorBeginOverlap
  (params (OtherActor :type Actor%20Object%20Reference)))

(event EventTick
  (params (DeltaSeconds :type Float%20%28single-precision%29)))

(event Input|KeyboardEvents|P
  (params (Key :type Key%20Structure :default "None"))
  (bind _returnvalue (Game|GetPlayerController 0))
  (:Pressed
    (Utilities|IsValid (Variables|Default|GetPauseMenuRef)
      (:Is%20Valid
        _)
      (:Is%20Not%20Valid
        (bind _returnvalue_2 (UserInterface|CreateWidget "/Game/UI/WBP_PauseMenu.WBP_PauseMenu_C"))
        (Variables|Default|SetPauseMenuRef _returnvalue_2)))
    (Variables|/Script/Engine.PlayerController|SetbShowMouseCursor _returnvalue true)
    (Input|SetInputModeUIOnly _returnvalue (Variables|Default|GetPauseMenuRef) "DoNotLock" false)
    (UserInterface|Viewport|AddtoViewport (Variables|Default|GetPauseMenuRef) 0)
    (Game|SetGamePaused true)))

(fn ConstructionScript)